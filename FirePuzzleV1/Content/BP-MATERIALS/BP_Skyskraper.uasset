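; Skyscraper building Blueprint that randomizes its color scheme for visual variety.
; The construction script picks one of four palettes (yellow, cream, blue, red) with an unseeded random integer and assigns materials to the mesh's named slots.
; Palettes override different sets of slots, and the pillar slot name alternates between "pillar" and "pillars".
; The event graph is empty, and one "frames" material assignment never runs.
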(fn `UserConstructionScript`
  (bind _mesh (`self.Mesh`))
  (switch `int` (`KismetMathLibrary.RandomInteger` 4)
    (:`0`
      ;[0.8625 0.6595 0.08266] yellow
      (`PrimitiveComponent.SetMaterialByName` _mesh "wall" "/Game/Materials/cream.cream")
      (`PrimitiveComponent.SetMaterialByName` _mesh "roofs" "/Game/Materials/yellow.yellow")
      (`PrimitiveComponent.SetMaterialByName` _mesh "pillar" "/Game/Materials/white.white"))
    (:`1`
      ;[1 0.7486 0.4658] cream
      (`PrimitiveComponent.SetMaterialByName` _mesh "wall" "/Game/Materials/yellow.yellow")
      (`PrimitiveComponent.SetMaterialByName` _mesh "roofs" "/Game/Materials/cream.cream")
      (`PrimitiveComponent.SetMaterialByName` _mesh "pillar" "/Game/Materials/cream.cream")
      (`PrimitiveComponent.SetMaterialByName` _mesh "plateau" "/Game/Materials/cream.cream")
      (`PrimitiveComponent.SetMaterialByName` _mesh "frame inside" "/Game/Materials/cream_darker.cream_darker"))
    (:`2`
      ;[0.2949 0.6201 1] blue
      (`PrimitiveComponent.SetMaterialByName` _mesh "wall" "/Game/Materials/blue.blue")
      (`PrimitiveComponent.SetMaterialByName` _mesh "roofs" "/Game/Materials/gray.gray")
      (`PrimitiveComponent.SetMaterialByName` _mesh "pillars" "/Game/Materials/cream.cream")
      (`PrimitiveComponent.SetMaterialByName` _mesh "plateau" "/Game/Materials/gray_darker.gray_darker")
      (`PrimitiveComponent.SetMaterialByName` _mesh "vent" "/Game/Materials/cream.cream")
      (`PrimitiveComponent.SetMaterialByName` _mesh "pipes" "/Game/Materials/gray_darker.gray_darker")
      (`PrimitiveComponent.SetMaterialByName` _mesh "frame inside" "/Game/Materials/gray_dark.gray_dark"))
    (:`3`
      ;[1 0.07396 0.07396] red
      (`PrimitiveComponent.SetMaterialByName` _mesh "wall" "/Game/Materials/red.red")
      (`PrimitiveComponent.SetMaterialByName` _mesh "roofs" "/Game/Materials/cream.cream")
      (`PrimitiveComponent.SetMaterialByName` _mesh "pillars" "/Game/Materials/white.white")
      (`PrimitiveComponent.SetMaterialByName` _mesh "plateau" "/Game/Materials/cream.cream")
      (`PrimitiveComponent.SetMaterialByName` _mesh "frame inside" "/Game/Materials/brown.brown")
      (`PrimitiveComponent.SetMaterialByName` _mesh "pipes" "/Game/Materials/gray_darker.gray_darker")
      (`PrimitiveComponent.SetMaterialByName` _mesh "vent" "/Game/Materials/gray.gray"))))