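; Small shed prop Blueprint that gives its mesh one of four random color schemes: brown, yellow, blue or red.
; The Construction Script rolls an unseeded random integer and sets materials by slot name, so the scheme can change whenever the script reruns.
; All schemes set wall, roofs and wood, while only some also override vent, frames or pillar.
; The event graph has no active logic.
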(fn `UserConstructionScript`
  (bind _mesh (`self.Mesh`))
  (switch `int` (`KismetMathLibrary.RandomInteger` 4)
    (:`0`
      ;[1 0.322 0.1313] brown
      (`PrimitiveComponent.SetMaterialByName` _mesh "wall" "/Game/Materials/tree_brown.tree_brown")
      (`PrimitiveComponent.SetMaterialByName` _mesh "roofs" "/Game/Materials/cream.cream")
      (`PrimitiveComponent.SetMaterialByName` _mesh "wood" "/Game/Materials/brown.brown"))
    (:`1`
      ;[1 0.7486 0.4658] yellow
      (`PrimitiveComponent.SetMaterialByName` _mesh "wall" "/Game/Materials/yellow.yellow")
      (`PrimitiveComponent.SetMaterialByName` _mesh "roofs" "/Game/Materials/cream_darker.cream_darker")
      (`PrimitiveComponent.SetMaterialByName` _mesh "wood" "/Game/Materials/brown.brown")
      (`PrimitiveComponent.SetMaterialByName` _mesh "vent" "/Game/Materials/white.white")
      (`PrimitiveComponent.SetMaterialByName` _mesh "frames" "/Game/Materials/cream.cream"))
    (:`2`
      ;[0.2949 0.6201 1] blue
      (`PrimitiveComponent.SetMaterialByName` _mesh "wall" "/Game/Materials/blue.blue")
      (`PrimitiveComponent.SetMaterialByName` _mesh "roofs" "/Game/Materials/gray_medium.gray_medium")
      (`PrimitiveComponent.SetMaterialByName` _mesh "pillar" "/Game/Materials/gray_darker.gray_darker")
      (`PrimitiveComponent.SetMaterialByName` _mesh "wood" "/Game/Materials/cream.cream"))
    (:`3`
      ;[1 0.07396 0.07396] red
      (`PrimitiveComponent.SetMaterialByName` _mesh "wall" "/Game/Materials/red.red")
      (`PrimitiveComponent.SetMaterialByName` _mesh "roofs" "/Game/Materials/cream.cream")
      (`PrimitiveComponent.SetMaterialByName` _mesh "wood" "/Game/Materials/brown_dark_2.brown_dark_2"))))