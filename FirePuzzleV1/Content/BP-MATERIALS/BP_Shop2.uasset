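; Shop building Blueprint that varies its look by assigning one of four random color schemes to its mesh.
; The Construction Script rolls a random integer and sets materials by slot name for a brown, cream, blue or red palette, with no seed.
; Palettes cover different slots, and the billboard hold slot name is spelled differently between them.
; The event graph is empty, and a frames material node is left unconnected.
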(fn `UserConstructionScript`
  (bind _mesh (`self.Mesh`))
  (switch `int` (`KismetMathLibrary.RandomInteger` 4)
    (:`0`
      ;[1 0.322 0.1313] brown
      (`PrimitiveComponent.SetMaterialByName` _mesh "wall" "/Game/Materials/tree_brown.tree_brown")
      (`PrimitiveComponent.SetMaterialByName` _mesh "roofs" "/Game/Materials/cream.cream")
      (`PrimitiveComponent.SetMaterialByName` _mesh "pillar" "/Game/Materials/cream.cream")
      (`PrimitiveComponent.SetMaterialByName` _mesh "wood" "/Game/Materials/cream.cream")
      (`PrimitiveComponent.SetMaterialByName` _mesh "billboard border " "/Game/Materials/white.white")
      (`PrimitiveComponent.SetMaterialByName` _mesh "billhold " "/Game/Materials/red.red"))
    (:`1`
      ;[1 0.7486 0.4658] cream
      (`PrimitiveComponent.SetMaterialByName` _mesh "wall" "/Game/Materials/cream.cream")
      (`PrimitiveComponent.SetMaterialByName` _mesh "roofs" "/Game/Materials/yellow.yellow")
      (`PrimitiveComponent.SetMaterialByName` _mesh "pillar" "/Game/Materials/tree_brown.tree_brown")
      (`PrimitiveComponent.SetMaterialByName` _mesh "wood" "/Game/Materials/brown_dark_2.brown_dark_2")
      (`PrimitiveComponent.SetMaterialByName` _mesh "vent" "/Game/Materials/white.white"))
    (:`2`
      ;[0.2949 0.6201 1] blue
      (`PrimitiveComponent.SetMaterialByName` _mesh "wall" "/Game/Materials/blue.blue")
      (`PrimitiveComponent.SetMaterialByName` _mesh "roofs" "/Game/Materials/gray.gray")
      (`PrimitiveComponent.SetMaterialByName` _mesh "pillar" "/Game/Materials/gray_darker.gray_darker")
      (`PrimitiveComponent.SetMaterialByName` _mesh "wood" "/Game/Materials/cream.cream")
      (`PrimitiveComponent.SetMaterialByName` _mesh "vent" "/Game/Materials/cream.cream")
      (`PrimitiveComponent.SetMaterialByName` _mesh "pipes" "/Game/Materials/gray_dark.gray_dark")
      (`PrimitiveComponent.SetMaterialByName` _mesh "billboard border" "/Game/Materials/gray_darker.gray_darker")
      (`PrimitiveComponent.SetMaterialByName` _mesh "billboard hold" "/Game/Materials/gray_dark.gray_dark"))
    (:`3`
      ;[1 0.07396 0.07396] red
      (`PrimitiveComponent.SetMaterialByName` _mesh "wall" "/Game/Materials/red.red")
      (`PrimitiveComponent.SetMaterialByName` _mesh "roofs" "/Game/Materials/cream.cream")
      (`PrimitiveComponent.SetMaterialByName` _mesh "pillar" "/Game/Materials/white.white")
      (`PrimitiveComponent.SetMaterialByName` _mesh "wood" "/Game/Materials/white.white")
      (`PrimitiveComponent.SetMaterialByName` _mesh "vent" "/Game/Materials/gray.gray")
      (`PrimitiveComponent.SetMaterialByName` _mesh "pipes" "/Game/Materials/gray_dark.gray_dark")
      (`PrimitiveComponent.SetMaterialByName` _mesh "billboard border" "/Game/Materials/white.white")
      (`PrimitiveComponent.SetMaterialByName` _mesh "billboard_hold " "/Game/Materials/cream.cream"))))