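; Big stable building Blueprint that randomizes the color scheme of its Shop mesh component.
; The construction script picks one of brown, yellow, blue or red and assigns materials by slot name to walls, frames and roofs.
; Each scheme overrides only some slots, and yellow targets "wall" where the others use "walls" and "wall2".
; The event graph has no active logic.
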(fn `UserConstructionScript`
  (bind _shop (`self.Shop`))
  (switch `int` (`KismetMathLibrary.RandomInteger` 4)
    (:`0`
      ;[1 0.322 0.1313] brown
      (`PrimitiveComponent.SetMaterialByName` _shop "walls" "/Game/materials/tree_brown.tree_brown")
      (`PrimitiveComponent.SetMaterialByName` _shop "frames" "/Game/materials/white.white")
      (`PrimitiveComponent.SetMaterialByName` _shop "wall2" "/Game/materials/tree_brown.tree_brown"))
    (:`1`
      ;[1 0.5482 0.1157] yellow
      (`PrimitiveComponent.SetMaterialByName` _shop "wall" "/Game/materials/yellow.yellow")
      (`PrimitiveComponent.SetMaterialByName` _shop "roofs" "/Game/materials/cream_darker.cream_darker")
      (`PrimitiveComponent.SetMaterialByName` _shop "frames" "/Game/materials/white.white"))
    (:`2`
      ;[0.2949 0.6201 1] blue
      (`PrimitiveComponent.SetMaterialByName` _shop "walls" "/Game/materials/blue.blue")
      (`PrimitiveComponent.SetMaterialByName` _shop "wall2" "/Game/materials/blue.blue")
      (`PrimitiveComponent.SetMaterialByName` _shop "roofs" "/Game/materials/gray_medium.gray_medium"))
    (:`3`
      ;[1 0.07396 0.07396] red
      (`PrimitiveComponent.SetMaterialByName` _shop "walls" "/Game/materials/red.red")
      (`PrimitiveComponent.SetMaterialByName` _shop "roofs" "/Game/materials/cream.cream")
      (`PrimitiveComponent.SetMaterialByName` _shop "wall2" "/Game/materials/red.red")
      (`PrimitiveComponent.SetMaterialByName` _shop "frames" "/Game/materials/white.white"))))