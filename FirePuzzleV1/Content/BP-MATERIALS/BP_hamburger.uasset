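; Hamburger building prop that gets a random color scheme for its static mesh.
; The Construction Script picks one of four palettes (blue, yellow, pink, red) and assigns materials to named slots such as wall, roofs, hood and balk.
; Palettes cover different slot sets, and unassigned slots are left untouched.
; The random pick is unseeded, and the event graph holds no active logic.
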(fn `UserConstructionScript`
  (bind _mesh (`self.Mesh`))
  (switch `int` (`KismetMathLibrary.RandomInteger` 4)
    (:`0`
      ;[0.09607 0.2351 0.5802] blue
      (`PrimitiveComponent.SetMaterialByName` _mesh "wall" "/Game/Materials/blue.blue")
      (`PrimitiveComponent.SetMaterialByName` _mesh "roofs" "/Game/Materials/cream.cream")
      (`PrimitiveComponent.SetMaterialByName` _mesh "hood" "/Game/Materials/blue_dark.blue_dark")
      (`PrimitiveComponent.SetMaterialByName` _mesh "roof frame" "/Game/Materials/cream.cream")
      (`PrimitiveComponent.SetMaterialByName` _mesh "frame inside" "/Game/Materials/glass.glass")
      (`PrimitiveComponent.SetMaterialByName` _mesh "balk" "/Game/Materials/gray_dark.gray_dark"))
    (:`1`
      ;[1 0.7486 0.4658] yellow
      (`PrimitiveComponent.SetMaterialByName` _mesh "wall" "/Game/Materials/yellow.yellow")
      (`PrimitiveComponent.SetMaterialByName` _mesh "roofs" "/Game/Materials/cream.cream")
      (`PrimitiveComponent.SetMaterialByName` _mesh "roof frame" "/Game/Materials/cream.cream")
      (`PrimitiveComponent.SetMaterialByName` _mesh "frame inside" "/Game/Materials/tree_brown.tree_brown")
      (`PrimitiveComponent.SetMaterialByName` _mesh "hood" "/Game/Materials/white.white")
      (`PrimitiveComponent.SetMaterialByName` _mesh "balk" "/Game/Materials/cream.cream"))
    (:`2`
      ;[1 0.4339 0.5789] pink
      (`PrimitiveComponent.SetMaterialByName` _mesh "wall" "/Game/Materials/pink.pink")
      (`PrimitiveComponent.SetMaterialByName` _mesh "roofs" "/Game/Materials/white.white")
      (`PrimitiveComponent.SetMaterialByName` _mesh "roof frame" "/Game/Materials/white.white")
      (`PrimitiveComponent.SetMaterialByName` _mesh "frame inside" "/Game/Materials/gray.gray")
      (`PrimitiveComponent.SetMaterialByName` _mesh "hood" "/Game/Materials/gray.gray")
      (`PrimitiveComponent.SetMaterialByName` _mesh "pipes" "/Game/Materials/gray.gray")
      (`PrimitiveComponent.SetMaterialByName` _mesh "vent" "/Game/Materials/cream.cream")
      (`PrimitiveComponent.SetMaterialByName` _mesh "balk" "/Game/Materials/cream.cream"))
    (:`3`
      ;[1 0.07396 0.07396] red
      (`PrimitiveComponent.SetMaterialByName` _mesh "wall" "/Game/Materials/red.red")
      (`PrimitiveComponent.SetMaterialByName` _mesh "roofs" "/Game/Materials/cream.cream")
      (`PrimitiveComponent.SetMaterialByName` _mesh "roof frame" "/Game/Materials/cream.cream")
      (`PrimitiveComponent.SetMaterialByName` _mesh "balk" "/Game/Materials/cream.cream"))))