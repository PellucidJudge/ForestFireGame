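; Shop building actor that randomly picks one of four color schemes (yellow, brown, red or blue) for its mesh.
; The Construction Script rolls an unseeded random integer, so the scheme can change whenever construction reruns.
; Each branch sets materials by slot name on a different subset of parts such as walls, roofs, wood and trim.
; The event graph holds no active logic.
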(fn `UserConstructionScript`
  (bind _mesh (`self.Mesh`))
  (switch `int` (`KismetMathLibrary.RandomInteger` 4)
    (:`0`
      ;[1 0.7796 0.1073] yellow
      (`PrimitiveComponent.SetMaterialByName` _mesh "wall" null)
      (`PrimitiveComponent.SetMaterialByName` _mesh "roofs" null)
      (`PrimitiveComponent.SetMaterialByName` _mesh "pillar" null)
      (`PrimitiveComponent.SetMaterialByName` _mesh "wood" null)
      (`PrimitiveComponent.SetMaterialByName` _mesh "rfames" null)
      (`PrimitiveComponent.SetMaterialByName` _mesh "billboard hold" null))
    (:`1`
      ;[0.3083 0.2308 0.1436] brown
      (`PrimitiveComponent.SetMaterialByName` _mesh "wall" null)
      (`PrimitiveComponent.SetMaterialByName` _mesh "roofs" null)
      (`PrimitiveComponent.SetMaterialByName` _mesh "plateau" null)
      (`PrimitiveComponent.SetMaterialByName` _mesh "wood" null)
      (`PrimitiveComponent.SetMaterialByName` _mesh "vent" null)
      (`PrimitiveComponent.SetMaterialByName` _mesh "hood" null))
    (:`2`
      ;[0.8667 0.1271 0.07944] red
      (`PrimitiveComponent.SetMaterialByName` _mesh "wall" null)
      (`PrimitiveComponent.SetMaterialByName` _mesh "roofs" null)
      (`PrimitiveComponent.SetMaterialByName` _mesh "hood" null)
      (`PrimitiveComponent.SetMaterialByName` _mesh "wood" null)
      (`PrimitiveComponent.SetMaterialByName` _mesh "vent" null)
      (`PrimitiveComponent.SetMaterialByName` _mesh "pipes" null)
      (`PrimitiveComponent.SetMaterialByName` _mesh "plateau" null)
      (`PrimitiveComponent.SetMaterialByName` _mesh "billboard hold" null))
    (:`3`
      ;[0.5491 0.5624 1] blue
      (`PrimitiveComponent.SetMaterialByName` _mesh "wall" null)
      (`PrimitiveComponent.SetMaterialByName` _mesh "roofs" null)
      (`PrimitiveComponent.SetMaterialByName` _mesh "pillar" null)
      (`PrimitiveComponent.SetMaterialByName` _mesh "wood" null)
      (`PrimitiveComponent.SetMaterialByName` _mesh "hood" null)
      (`PrimitiveComponent.SetMaterialByName` _mesh "pipes" null)
      (`PrimitiveComponent.SetMaterialByName` _mesh "plateau" null)
      (`PrimitiveComponent.SetMaterialByName` _mesh "frames" null))))