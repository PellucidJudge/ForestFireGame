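; Spruce tree prop Blueprint that randomizes its look for placing varied trees in a level.
; The Construction Script picks one of five spruce static meshes at random for its Mesh component.
; A second coin flip either applies brown and green materials to the trunk and leaves slots or sets them with no material specified.
; Rolls are unseeded, so reconstruction can change the result, and the event graph is unused.
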(fn `UserConstructionScript`
  (bind _mesh (`self.Mesh`))
  (switch `int` (`KismetMathLibrary.RandomInteger` 5)
    (:`0`
      (`StaticMeshComponent.SetStaticMesh` _mesh "/Game/models/spruce2.spruce2"))
    (:`1`
      (`StaticMeshComponent.SetStaticMesh` (`self.Mesh`) "/Game/models/spruce3.spruce3"))
    (:`2`
      (`StaticMeshComponent.SetStaticMesh` (`self.Mesh`) "/Game/models/spruce4.spruce4"))
    (:`3`
      (`StaticMeshComponent.SetStaticMesh` (`self.Mesh`) "/Game/models/spruce5.spruce5"))
    (:`4`
      (`StaticMeshComponent.SetStaticMesh` (`self.Mesh`) "/Game/models/spruce_6.spruce_6")))
  (switch `int` (`KismetMathLibrary.RandomInteger` 2)
    (:`0`
      (`PrimitiveComponent.SetMaterialByName` _mesh "trunk" "/Game/Materials/brown.brown")
      (`PrimitiveComponent.SetMaterialByName` (`self.Mesh`) "trunk" "/Game/Materials/brown.brown")
      (`PrimitiveComponent.SetMaterialByName` (`self.Mesh`) "trunk" "/Game/Materials/brown.brown")
      (`PrimitiveComponent.SetMaterialByName` (`self.Mesh`) "trunk" "/Game/Materials/brown.brown")
      (`PrimitiveComponent.SetMaterialByName` (`self.Mesh`) "trunk" "/Game/Materials/brown.brown")
      (`PrimitiveComponent.SetMaterialByName` _mesh "leaves" "/Game/Materials/tree_green.tree_green")
      (`PrimitiveComponent.SetMaterialByName` (`self.Mesh`) "leaves" "/Game/Materials/tree_green.tree_green")
      (`PrimitiveComponent.SetMaterialByName` (`self.Mesh`) "leaves" "/Game/Materials/tree_green.tree_green")
      (`PrimitiveComponent.SetMaterialByName` (`self.Mesh`) "leaves" "/Game/Materials/tree_green.tree_green")
      (`PrimitiveComponent.SetMaterialByName` (`self.Mesh`) "leaves" "/Game/Materials/tree_green.tree_green"))
    (:`1`
      (`PrimitiveComponent.SetMaterialByName` _mesh "trunk" null)
      (`PrimitiveComponent.SetMaterialByName` (`self.Mesh`) "trunk" null)
      (`PrimitiveComponent.SetMaterialByName` (`self.Mesh`) "trunk" null)
      (`PrimitiveComponent.SetMaterialByName` (`self.Mesh`) "trunk" null)
      (`PrimitiveComponent.SetMaterialByName` (`self.Mesh`) "trunk" null)
      (`PrimitiveComponent.SetMaterialByName` _mesh "leaves" null)
      (`PrimitiveComponent.SetMaterialByName` (`self.Mesh`) "leaves" null)
      (`PrimitiveComponent.SetMaterialByName` (`self.Mesh`) "leaves" null)
      (`PrimitiveComponent.SetMaterialByName` (`self.Mesh`) "leaves" null)
      (`PrimitiveComponent.SetMaterialByName` (`self.Mesh`) "leaves" null))))