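; Fire starter Blueprint that scatters a number of child fire-start actors at random spots within a rectangular area.
; The construction script destroys previously spawned components, scales the area marker and box to the area size, then adds child actor components at random XY offsets centred on the actor.
; A seeded random stream drives placement, and at least one fire is always created.
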(fn `UserConstructionScript`
  (bind (_randomareasize_x _randomareasize_y) (`KismetMathLibrary.BreakVector2D` (`self.RandomAreaSize`)))
  (bind _firestartactors (`self.FirestartActors`))
  (bind (_randomareasize_x_2 _randomareasize_y_2) (`KismetMathLibrary.BreakVector2D` (`self.RandomAreaSize`)))
  (bind _seed (`self.Seed`))
  (bind _returnvalue (`KismetMathLibrary.MakeVector` _randomareasize_x _randomareasize_y 1.0))
  (`parent.UserConstructionScript`)
  (`|ExecutionSequence`
    (:`then_0`
      ;[1 1 1] Reset
      (for _array_element _firestartactors
        (`ActorComponent.K2_DestroyComponent` _array_element))
      (`KismetArrayLibrary.Array_Clear` _firestartactors))
    (:`then_1`
      ;[1 1 1] Editor visuals
      (`SceneComponent.SetRelativeScale3D` (`self.AreaMarker`) _returnvalue)
      (`SceneComponent.SetRelativeScale3D` (`self.Box`) _returnvalue))
    (:`then_2`
      (for _ (range (+ (`KismetMathLibrary.Max` (- (`self.NumberOfFires`) 1)) 1))
        (bind _returnvalue_2 (`AddComponent|NODE_AddChildActorComponent-0` :`RelativeTransform` (`KismetMathLibrary.MakeTransform` (`KismetMathLibrary.MakeVector` (- (`KismetMathLibrary.RandomFloatInRangeFromStream` 0.0 _randomareasize_x_2 _seed) (/ _randomareasize_x_2 2.0)) (- (`KismetMathLibrary.RandomFloatInRangeFromStream` 0.0 _randomareasize_y_2 _seed) (/ _randomareasize_y_2 2.0))))))
        (`KismetArrayLibrary.Array_Add` (`self.FirestartActors`) _returnvalue_2)))))