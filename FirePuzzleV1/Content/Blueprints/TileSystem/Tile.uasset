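; Tile in the tile system that stores its own fire state: resistance, burn time, and on-fire and burnt-out flags, plus a Value.
; Resistance changes are clamped between zero and a maximum.
; Ignition and burnout only set flags, and burn-time increments return current and maximum, leaving fire decisions to callers.
; A text render component displays a debug index with optional color.
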(event `self.ReceiveBeginPlay`)

(fn `AddFireResistance`
  (params (AddAmount :type "Float (double-precision)"))
  (returns (AddedFireRes :type "Float (double-precision)"))
  (locals (OldFireRes :type "Float (double-precision)"))
  (bind _fireresistancecurrent (`self.FireResistanceCurrent`))
  (bind _returnvalue (`KismetMathLibrary.FClamp` (+ AddAmount _fireresistancecurrent) 0.0 (`self.FireResistanceMax`)))
  (set `local.OldFireRes` _fireresistancecurrent)
  (set `self.FireResistanceCurrent` _returnvalue)
  (return (- _returnvalue (`local.OldFireRes`))))

(fn `DamageFireResistance`
  (params (FireResDamage :type "Float (double-precision)"))
  (returns (TotalDamage :type "Float (double-precision)"))
  (locals (OldFireRes :type "Float (double-precision)"))
  (bind _fireresistancecurrent (`self.FireResistanceCurrent`))
  (bind _returnvalue (`KismetMathLibrary.FClamp` (- _fireresistancecurrent FireResDamage) 0.0 (`self.FireResistanceMax`)))
  (set `local.OldFireRes` _fireresistancecurrent)
  (set `self.FireResistanceCurrent` _returnvalue)
  (return (- _returnvalue (`local.OldFireRes`))))

(fn `GetCurrentBurnTime`
  (returns (BurnTime :type Integer))
  (return (`self.BurnTimeCurrent`)))

(fn `GetFireResistance`
  (returns (FireRes :type "Float (double-precision)"))
  (return (`self.FireResistanceCurrent`)))

(fn `GetIsBurntOut`
  (returns (BurntOut :type Boolean))
  (return (`self.IsBurntOut`)))

(fn `GetIsOnFire`
  (returns (IsOnFire :type Boolean))
  (return (`self.IsOnFire`)))

(fn `IncrementBurnTime`
  (returns (NewBurnoutTime :type Integer) (MaxBurnoutTime :type Integer))
  (bind _result (`/Engine/EditorBlueprintResources/StandardMacros.IncrementInt` (`self.BurnTimeCurrent`))
    (:`  `
      (return _result (`self.BurnTimeMax`)))))

(fn `LightOnFire`
  (set `self.IsOnFire` true))

(fn `SetIndexDebug`
  (params (Text :type Text) (ChangeColor :type Boolean) (TextColor :type "Color Structure"))
  (bind _indexdebug (`self.IndexDebug`))
  (`TextRenderComponent.K2_SetText` _indexdebug Text)
  (if ChangeColor
    (`TextRenderComponent.SetTextRenderColor` _indexdebug TextColor)))

(fn `SetStartBurnTime`
  (params (BurnTime :type Integer))
  (set `self.BurnTimeMax` BurnTime))

(fn `SetStartFireResistance`
  (params (FireRes :type "Float (double-precision)"))
  (set `self.FireResistanceCurrent` (`KismetMathLibrary.FClamp` FireRes 0.0 (`self.FireResistanceMax`))))

(fn `SetValue`
  (params (Value :type "Float (double-precision)"))
  (set `self.Value` Value))

(fn `TileBurnout`
  (set `self.IsOnFire` false)
  (set `self.IsBurntOut` true))

(fn `UserConstructionScript`)