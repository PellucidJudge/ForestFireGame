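; Base chunk actor for a fire-spread tile system, holding a square grid of tiles and the flammable objects on it.
; The construction script builds Tile child actors, applies per-tile fire resistance, burn time and value from ChunkTilesData, and shows resistance as colored debug text.
; BeginPlay respawns Flammable_Base child actors as standalone tracked actors, destroying the originals.
; BurnFlammableObjects ignites tracked objects near a location; quench and burnout functions are empty stubs.
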(event `self.ReceiveBeginPlay`
  (bind _childactors (`self.GetAllChildActors` true))
  (for _array_element _childactors
    (bind _asflammable_base (cast `/Game/Blueprints/FlammableActors/Flammable_Base` _array_element))
    (bind _returnvalue (`|SpawnActorFromClass` (`GameplayStatics.GetObjectClass` _asflammable_base) (`SceneComponent.K2_GetComponentToWorld` (`/Game/Blueprints/FlammableActors/Flammable_Base.DefaultSceneRoot` _asflammable_base)) "AlwaysSpawn" "OverrideRootScale" null null))
    (bind _asflammable_base_2 (cast `/Game/Blueprints/FlammableActors/Flammable_Base` _returnvalue))
    (`KismetArrayLibrary.Array_AddUnique` (`self.FlammableObjects`) _asflammable_base_2))
  (for _array_element_2 _childactors
    (`/Engine/EditorBlueprintResources/StandardMacros.IsValid` _array_element_2
      (:`Is Valid`
        (bind _asflammable_base_3 (cast `/Game/Blueprints/FlammableActors/Flammable_Base` _array_element_2))
        (`self.K2_DestroyActor` _asflammable_base_3)))))

(fn `BurnFlammableObjects`
  (params (Location :type "Vector Structure") (CheckAreaSize :type "Float (double-precision)"))
  (locals (BurntObjects :type "Array of /Game/Blueprints/FlammableActors/Flammable_Base Object Reference"))
  (for _array_element (`self.FlammableObjects`)
    (if (== (`self.K2_GetActorLocation` _array_element) Location :`ErrorTolerance` CheckAreaSize)
      (`KismetArrayLibrary.Array_Add` (`local.BurntObjects`) _array_element)))
  (for _array_element_2 (`local.BurntObjects`)
    (`KismetArrayLibrary.Array_RemoveItem` (`self.FlammableObjects`) _array_element_2)
    (`/Game/Blueprints/FlammableActors/Flammable_Base.BurnObject` _array_element_2)
    (`KismetArrayLibrary.Array_AddUnique` (`self.BurningObjects`) _array_element_2)))

(fn `BurnoutObjects`)

(fn `QuenchBurningObjects`)

(fn `UserConstructionScript`
  (bind _chunksidelength (`self.ChunkSideLength`))
  (bind _chunksidelength_2 (`self.ChunkSideLength`))
  (bind _tilewidth (`self.TileWidth`))
  (`|ExecutionSequence`
    (:`then_0`
      ;[1 1 1] Create tiles
      (`KismetArrayLibrary.Array_Clear` (`self.TileArray`))
      (for _index (range (* _chunksidelength _chunksidelength))
        (bind _returnvalue (`AddComponent|NODE_AddChildActorComponent-0` :`RelativeTransform` (`KismetMathLibrary.MakeTransform` (`KismetMathLibrary.MakeVector` (* (mod _index _chunksidelength_2) _tilewidth) (* (/ _index _chunksidelength_2) _tilewidth)))))
        (bind _astile (cast `/Game/Blueprints/TileSystem/Tile` (`ChildActorComponent.ChildActor` _returnvalue)))
        (bind _returnvalue_2 (`KismetArrayLibrary.Array_Add` (`self.TileArray`) _astile))
        (bind _fireres (`/Game/Blueprints/TileSystem/Tile.GetFireResistance` _astile))
        (`/Game/Blueprints/TileSystem/Tile.SetIndexDebug` _astile (`KismetTextLibrary.Conv_StringToText` (`KismetStringLibrary.Concat_StrStr` "" (`KismetStringLibrary.Conv_IntToString` (`KismetMathLibrary.FTrunc` _fireres)))) true (make `Color` 0 (* (`KismetMathLibrary.Conv_IntToByte` _returnvalue_2) 2)))))
    (:`then_1`
      ;[1 1 1] Set tile values
      (if (== (`KismetArrayLibrary.Array_Length` (`self.TileArray`)) (`KismetArrayLibrary.Array_Length` (`self.ChunkTilesData`)))
        (for (_array_element _array_index) (`self.TileArray`)
          (bind (_fireresistance _burntime _value) (break `/Game/Blueprints/TileSystem/TileDataStruct` (`|GetArrayItem` (`self.ChunkTilesData`) _array_index)))
          (`/Game/Blueprints/TileSystem/Tile.SetStartFireResistance` _array_element _fireresistance)
          (`/Game/Blueprints/TileSystem/Tile.SetStartBurnTime` _array_element _burntime)
          (`/Game/Blueprints/TileSystem/Tile.SetValue` _array_element _value)
          (bind _fireres_2 (`/Game/Blueprints/TileSystem/Tile.GetFireResistance` _array_element))
          (`/Game/Blueprints/TileSystem/Tile.SetIndexDebug` _array_element (`KismetTextLibrary.Conv_StringToText` (`KismetStringLibrary.Concat_StrStr` "" (`KismetStringLibrary.Conv_IntToString` (`KismetMathLibrary.FTrunc` _fireres_2)))) true (`KismetMathLibrary.Conv_LinearColorToColor` (`KismetMathLibrary.LinearColorLerp` (struct :`R` 0.254167 :`A` 1.0) (struct :`R` 0.010966 :`G` 0.170833 :`A` 1.0) (/ _fireres_2 100.0)))))))))